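; Base character Blueprint that delegates health, damage, healing and death state to a DamageSystem component through wrapper functions.
; The component's damage, heal and death events route to Respond events, with damage and heal printing debug text.
; RespondToHeal also calls HandleIncomingHeal on the component, although it is itself triggered by OnHealReceived.
; Death disables capsule collision and ragdolls the mesh with physics simulation.
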(event OnDamageTaken(DamageSystem)
  (params (DamageInfo :type Damage%20Info%20Structure%20%28by%20ref%29))
  (CallFunction|RespondtoDamageTaken DamageInfo))

(event OnDeath(DamageSystem)
  (CallFunction|RespondtoDeath))

(event OnHealReceived(DamageSystem)
  (params (HealAmount :type Float%20%28single-precision%29) (Healer :type Actor%20Object%20Reference))
  (CallFunction|RespondtoHeal HealAmount Healer))

(event Custom|RespondToDeath
  (bind _mesh (Variables|Character|GetMesh))
  (Collision|SetCollisionEnabled (Variables|Collision|GetCapsuleComponent) "NoCollision")
  (Collision|SetCollisionEnabled _mesh "QueryAndPhysics")
  (Physics|SetSimulatePhysics _mesh true))

(event Custom|RespondToDamageTaken
  (params (DamageInfo :type Damage%20Info%20Structure))
  (bind (_damageamount _damagecauser) (Utilities|Struct|BreakDamageInfo DamageInfo))
  (Development|PrintString (Utilities|String|Append (Utilities|String|ToString(Float) _damageamount) "  Damage by " (Utilities|GetDisplayName _damagecauser))))

(event Custom|RespondToHeal
  (params (HealAmount :type Float%20%28single-precision%29) (Healer :type Actor%20Object%20Reference))
  (bind _damagesystem (Variables|Default|GetDamageSystem))
  (Class|DamageSystemComponent|HandleIncomingHeal _damagesystem HealAmount Healer)
  (Development|PrintString (Utilities|String|ToString(Float) (Class|DamageSystemComponent|GetCurrentHealth _damagesystem))))

(fn ConstructionScript)

(fn TakeDamage
  (params (DamageInfo :type Damage%20Info%20Structure%20%28by%20ref%29))
  (bind _returnvalue (Class|DamageSystemComponent|HandleIncomingDamage (Variables|Default|GetDamageSystem) DamageInfo))
  (return _returnvalue))

(fn GetMaxHealth
  (return (Class|DamageSystemComponent|GetMaxHealth (Variables|Default|GetDamageSystem))))

(fn GetIsDead
  (return (Class|DamageSystemComponent|GetIsDead (Variables|Default|GetDamageSystem))))

(fn GetCurrentHealth
  (return (Class|DamageSystemComponent|GetCurrentHealth (Variables|Default|GetDamageSystem))))